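; BP_BarrelEvidence is a barrel evidence objective that reacts to being photographed with the camera flash.
; On BeginPlay it creates dynamic material instances from the mesh's two slots, one opaque and one translucent.
; A valid flash photo swaps slot 0 to the translucent instance while a timeline drives its opacity, then restores the opaque one.
; The same photo reports the barrel evidence tag to the photographing character.
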(event EventBeginPlay
  (|CallParentFunction)
  (bind _returnvalue (Rendering|Material|CreateDynamicMaterialInstance (Variables|Character|GetMesh) 0 0 "None" :!class /Script/Engine.PrimitiveComponent))
  (Variables|Default|SetOpaque _returnvalue)
  (bind _returnvalue_2 (Rendering|Material|CreateDynamicMaterialInstance (Variables|Character|GetMesh) 1 0 "None" :!class /Script/Engine.PrimitiveComponent))
  (Variables|Default|SetTranslucent _returnvalue_2))

(event Collision|EventActorBeginOverlap
  (params (OtherActor :type Actor%20Object%20Reference)))

(event EventTick
  (params (DeltaSeconds :type Float%20%28single-precision%29)))

(event EventOnEvidencePhotographed
  (params (PhotographingCharacter :type Stealth%20Detective%20Game%20Character%20Object%20Reference))
  (if (and (Class|StealthDetectiveGameCharacter|GetIsCameraFlashEnabled PhotographingCharacter) (Variables|/Script/StealthDetectiveGame.StealthDetectiveGameCharacter|GetbCanFlash PhotographingCharacter))
    (Utilities|FlowControl|Sequence
      (:then_0
        (Rendering|Material|SetMaterial (Variables|Character|GetMesh) 0 (Variables|Default|GetTranslucent))
        (bind _opacity (Timeline|FlashTimeline PlayFromStart)
          (:Update
            (Rendering|Material|SetScalarParameterValue (Variables|Default|GetTranslucent) "OpacityAmount" _opacity :!class /Script/Engine.MaterialInstanceDynamic))
          (:Finished
            (Rendering|Material|SetMaterial (Variables|Character|GetMesh) 0 (Variables|Default|GetOpaque)))))
      (:then_1
        (Default|CallOnEvidenceFound PhotographingCharacter "(TagName=\"Evidence.Objective.Barrel\")")))))

(fn ConstructionScript
  (|CallParentFunction))