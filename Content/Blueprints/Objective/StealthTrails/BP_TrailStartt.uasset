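; BP_TrailStartt is a stealth trail objective actor that pairs a configurable mesh with a colored Niagara gas effect tied to detective vision.
; The construction script applies ObjectMesh to the mesh component.
; BeginPlay flips the gas's visibility from its default, then passes NiagaraColor to the effect's Color parameter.
; The IA_EnableDetectiveVision input event toggles the gas visibility, including child components, rather than setting an explicit state.
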(event Input|EnhancedActionEvents|EnhancedInputActionIA_EnableDetectiveVision
  (params (ActionValue :type Boolean) (ElapsedSeconds :type Float%20%28double-precision%29) (TriggeredSeconds :type Float%20%28double-precision%29) (InputAction :type Input%20Action%20Object%20Reference :default "/Game/Input/Actions/Default/IA_EnableDetectiveVision.IA_EnableDetectiveVision"))
  (Rendering|ToggleVisibility (Variables|Default|GetGas) true))

(event EventBeginPlay
  (Utilities|FlowControl|Sequence
    (:then_0
      (Rendering|ToggleVisibility (Variables|Default|GetGas) true))
    (:then_1
      (Niagara|SetNiagaraVariable(LinearColor) (Variables|Default|GetGas) "Color" (Variables|Default|GetNiagaraColor)))))

(event Collision|EventActorBeginOverlap
  (params (OtherActor :type Actor%20Object%20Reference)))

(event EventTick
  (params (DeltaSeconds :type Float%20%28single-precision%29)))

(fn ConstructionScript
  (Components|StaticMesh|SetStaticMesh (Variables|Default|GetMesh) (Variables|Default|GetObjectMesh)))