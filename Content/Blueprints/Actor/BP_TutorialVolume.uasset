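; BP_TutorialVolume is a trigger volume that shows an on-screen tutorial prompt while the player character is inside it.
; Box overlap begin creates a WBP_TutorialText widget for the character's controller, filled with configurable prefix and suffix text plus keyboard and gamepad icons.
; The initial icon follows the current CommonInput input type.
; Overlap end removes the widget and forces garbage collection.
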(event Custom|OnComponentEndOverlap_Event
  (params (OverlappedComponent :type Primitive%20Component%20Object%20Reference) (OtherActor :type Actor%20Object%20Reference) (OtherComp :type Primitive%20Component%20Object%20Reference) (OtherBodyIndex :type Integer))
  (CallFunction|HideTutorialText OtherActor))

(event Custom|OnComponentBeginOverlap_Event
  (params (OverlappedComponent :type Primitive%20Component%20Object%20Reference) (OtherActor :type Actor%20Object%20Reference) (OtherComp :type Primitive%20Component%20Object%20Reference) (OtherBodyIndex :type Integer) (bFromSweep :type Boolean) (SweepResult :type Hit%20Result%20Structure%20%28by%20ref%29))
  (CallFunction|ShowTutorialText OtherActor))

(event EventBeginPlay
  (bind _box (Variables|Default|GetBox))
  (Collision|AssignOnComponentBeginOverlap _box (delegate Custom|OnComponentBeginOverlap_Event))
  (Collision|AssignOnComponentEndOverlap _box (delegate Custom|OnComponentEndOverlap_Event)))

(event Collision|EventActorBeginOverlap
  (params (OtherActor :type Actor%20Object%20Reference)))

(event EventTick
  (params (DeltaSeconds :type Float%20%28single-precision%29)))

(fn ConstructionScript)

(fn ShowTutorialText
  (params (InActor :type Actor%20Object%20Reference))
  (bind _asbp_third_person_character (Utilities|Casting|CastToBP_ThirdPersonCharacter InActor))
  (bind _asbp_third_person_player_controller (Utilities|Casting|CastToBP_ThirdPersonPlayerController (Pawn|GetController _asbp_third_person_character)))
  (bind _returnvalue (UserInterface|CreateWidget "/Game/Blueprints/UI/WBP_TutorialText.WBP_TutorialText_C" _asbp_third_person_player_controller))
  (bind _output_get (Variables|Default|SetTutorialTextWidget _returnvalue))
  (CallFunction|SetupTutorialTextWidget _output_get _asbp_third_person_player_controller)
  (UserInterface|Viewport|AddtoViewport _output_get 0))

(fn HideTutorialText
  (params (InActor :type Actor%20Object%20Reference))
  (bind _tutorialtextwidget (Variables|Default|GetTutorialTextWidget))
  (bind _asbp_third_person_character (Utilities|Casting|CastToBP_ThirdPersonCharacter InActor))
  (Utilities|Casting|CastToBP_ThirdPersonPlayerController (Pawn|GetController _asbp_third_person_character))
  (Utilities|IsValid _tutorialtextwidget
    (:Is%20Valid
      (Widget|RemovefromParent _tutorialtextwidget)
      (Utilities|Platform|CollectGarbage))))

(fn SetupTutorialTextWidget
  (params (InWidget :type WBP%20Tutorial%20Text%20Object%20Reference) (PlayerController :type Player%20Controller%20Object%20Reference))
  (bind _iconimage (Variables|/Game/Blueprints/UI/WBP_TutorialText.WBP_TutorialText_C|GetIconImage InWidget))
  (Rendering|Components|TextRender|SetText (Variables|/Game/Blueprints/UI/WBP_TutorialText.WBP_TutorialText_C|GetPrefix_Text InWidget) (Variables|Default|GetPrefixPrompt))
  (Rendering|Components|TextRender|SetText (Variables|/Game/Blueprints/UI/WBP_TutorialText.WBP_TutorialText_C|GetSuffix_Text InWidget) (Variables|Default|GetSuffixPrompt))
  (Variables|/Game/Blueprints/UI/WBP_TutorialText.WBP_TutorialText_C|SetIconImageGamepad InWidget (Variables|Default|GetIconGamepad))
  (Variables|/Game/Blueprints/UI/WBP_TutorialText.WBP_TutorialText_C|SetIconImagePC InWidget (Variables|Default|GetIconKeyboard))
  (switch Utilities|FlowControl|Switch|SwitchonECommonInputType (Class|CommonInputSubsystem|GetCurrentInputType (PlayerController|LocalPlayerSubsystems|GetCommonInputSubsystem PlayerController))
    (:MouseAndKeyboard
      (Class|Image|SetBrush _iconimage (Utilities|Struct|MakeSlateBrush "(SpecifiedColor=(R=1.000000,G=1.000000,B=1.000000,A=1.000000),ColorUseRule=UseColor_Specified)" "Image" "NoTile" "NoMirror" "(X=32.000000,Y=32.000000)" "(Left=0.000000,Top=0.000000,Right=0.000000,Bottom=0.000000)" (Variables|Default|GetIconKeyboard) "(CornerRadii=(X=0.000000,Y=0.000000,Z=0.000000,W=0.000000),Color=(SpecifiedColor=(R=0.000000,G=0.000000,B=0.000000,A=0.000000),ColorUseRule=UseColor_Specified),Width=0.000000,RoundingType=HalfHeightRadius,bUseBrushTransparency=False)")))
    (:Gamepad
      (Class|Image|SetBrush _iconimage (Utilities|Struct|MakeSlateBrush "(SpecifiedColor=(R=1.000000,G=1.000000,B=1.000000,A=1.000000),ColorUseRule=UseColor_Specified)" "Image" "NoTile" "NoMirror" "(X=32.000000,Y=32.000000)" "(Left=0.000000,Top=0.000000,Right=0.000000,Bottom=0.000000)" (Variables|Default|GetIconGamepad) "(CornerRadii=(X=0.000000,Y=0.000000,Z=0.000000,W=0.000000),Color=(SpecifiedColor=(R=0.000000,G=0.000000,B=0.000000,A=0.000000),ColorUseRule=UseColor_Specified),Width=0.000000,RoundingType=HalfHeightRadius,bUseBrushTransparency=False)")))))