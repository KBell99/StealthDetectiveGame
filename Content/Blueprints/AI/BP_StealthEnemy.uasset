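; Stealth enemy character that carries a spawned flashlight in its right hand and reports sightings of the player to a State Tree.
; AI perception updates PlayerInSight and, on detection, sends an event through BP_StealthAIController with the player and location as an instanced-struct payload.
; TreeSucceeded sends a PlayerDead event to the same tree.
; Overlapping a closed stealth door opens it, and Foley functions enable footstep sounds.
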(event OnTargetPerceptionUpdated(AIPerceptionComponent)
  (params (Actor :type Actor%20Object%20Reference) (Stimulus :type AI%20Stimulus%20Structure))
  (bind _asbp_third_person_character (Utilities|Casting|CastToBP_ThirdPersonCharacter Actor))
  (if (.bsuccessfullysensed Stimulus)
    (Variables|Default|SetbPlayerInSight true)
    (bind _asbp_stealth_aicontroller (Utilities|Casting|CastToBP_StealthAIController (Pawn|GetController)))
    (bind _returnvalue (Utilities|InstancedStruct|MakeInstancedStruct (Utilities|Struct|MakePlayerLocationInfo _asbp_third_person_character (Transformation|GetActorLocation _asbp_third_person_character) (Utilities|Time|GetWorldDeltaSeconds))))
    (Gameplay|StateTree|SendStateTreeEvent (Variables|/Script/StealthDetectiveGame.StealthAIController|GetStateTreeAI _asbp_stealth_aicontroller) (Utilities|Struct|MakeStateTreeEvent "(TagName=\"Status.PlayerInSight\")" _returnvalue "Character") :!class /Script/GameplayStateTreeModule.StateTreeComponent)
    (else
      (Variables|Default|SetbPlayerInSight false))))

(event EventBeginPlay
  (bind _returnvalue (Game|SpawnActorfromClass "/Game/Blueprints/Actor/BP_Flashlight.BP_Flashlight_C" (Transformation|GetActorTransform) "Undefined" "MultiplyWithRoot" 0 0))
  (bind _output_get (Variables|Default|SetFlashlight _returnvalue))
  (Transformation|AttachComponentToComponent _output_get (Variables|Character|GetMesh) "HandGrip_R" "SnapToTarget" "SnapToTarget" "SnapToTarget" true))

(event EventTreeSucceeded
  (params (DeadCharacter :type Stealth%20Detective%20Game%20Character%20Object%20Reference))
  (bind _asbp_stealth_aicontroller (Utilities|Casting|CastToBP_StealthAIController (Pawn|GetController)))
  (Gameplay|StateTree|SendStateTreeEvent (Variables|/Script/StealthDetectiveGame.StealthAIController|GetStateTreeAI _asbp_stealth_aicontroller) (Utilities|Struct|MakeStateTreeEvent "(TagName=\"Status.PlayerDead\")" "None" "Character") :!class /Script/GameplayStateTreeModule.StateTreeComponent))

(event EventTick
  (params (DeltaSeconds :type Float%20%28single-precision%29)))

(event Collision|EventActorBeginOverlap
  (params (OtherActor :type Actor%20Object%20Reference))
  (bind _asbp_stealth_door (Utilities|Casting|CastToBP_StealthDoor OtherActor))
  (if (not (Variables|/Game/Blueprints/Actor/BP_StealthDoor.BP_StealthDoor_C|GetIsDoorOpen _asbp_stealth_door))
    (Class|Interactable|OnInteract _asbp_stealth_door self)))

(fn ConstructionScript)

(fn CanPlayFootstepSounds
  (return true))

(fn GetFoleyAudioBank
  (return "/Game/Assets/Audio/Foley/DefaultFoleyEventAudioBank.DefaultFoleyEventAudioBank"))